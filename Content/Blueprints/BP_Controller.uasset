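; Player controller logic for a BP_Camera pawn, cached on BeginPlay with its spring arm and movement component.
; Forward/back sets location along camera facing at fixed height with a speed modifier; left/right feeds world-Y movement input.
; Zoom clamps arm length; holding Pan opens gates letting mouse axes drive yaw and pitch, with resets for zoom and pitch.
; A helper computes screen-edge scroll speeds, unused in these graphs.
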(event EventBeginPlay
  ;[1 1 1] Initialize (초기화)
  (bind _asbp_camera (Utilities|Casting|CastToBP_Camera (Game|Player|GetPlayerPawn 0)))
  (bind _output_get (Variables|Default|SetBP_Camera _asbp_camera))
  (Variables|Default|SetFloating%20Pawn%20Movement (Variables|/Game/Blueprints/BP_Camera.BP_Camera_C|GetFloatingPawnMovement _output_get))
  (Variables|Default|SetSpring%20Arm (Variables|/Game/Blueprints/BP_Camera.BP_Camera_C|GetSpringArm (Variables|Default|GetBP_Camera))))

(event Input|ActionEvents|InputActionZoomIn
  (params (Key :type Key%20Structure :default "None"))
  (bind _spring_arm (Variables|Default|GetSpring%20Arm))
  ;[1 1 1] 줌 인
  (:Pressed
    (Variables|/Script/Engine.SpringArmComponent|SetTargetArmLength _spring_arm (Math|Float|Clamp(Float) (- (Variables|/Script/Engine.SpringArmComponent|GetTargetArmLength _spring_arm) (Variables|Default|Get줌%20인/아웃%20스피드)) 5e+02 1.5e+03))))

(event Input|ActionEvents|InputActionZoomOut
  (params (Key :type Key%20Structure :default "None"))
  (bind _spring_arm (Variables|Default|GetSpring%20Arm))
  ;[1 1 1] 줌 아웃
  (:Pressed
    (Variables|/Script/Engine.SpringArmComponent|SetTargetArmLength _spring_arm (Math|Float|Clamp(Float) (+ (Variables|/Script/Engine.SpringArmComponent|GetTargetArmLength _spring_arm) (Variables|Default|Get줌%20인/아웃%20스피드)) 5e+02 1.5e+03))))

(event Input|ActionEvents|InputActionZoomReset
  (params (Key :type Key%20Structure :default "None"))
  ;[1 1 1] 줌 리셋
  (:Pressed
    (Variables|/Script/Engine.SpringArmComponent|SetTargetArmLength (Variables|Default|GetSpring%20Arm) (Variables|Default|Get타깃%20암%20길이))))

(event Input|ActionEvents|InputActionPan_Reset
  (params (Key :type Key%20Structure :default "None"))
  (bind _bp_camera (Variables|Default|GetBP_Camera))
  (bind _returnvalue (Transformation|GetActorRotation _bp_camera))
  (bind (_roll _pitch _yaw) (Math|Rotator|BreakRotator _returnvalue))
  ;[1 1 1] 팬 리셋
  (:Pressed
    (Transformation|SetActorRotation (Variables|Default|GetBP_Camera) (Math|Rotator|MakeRotator _roll 0.0 _yaw))))

(event Input|ActionEvents|InputActionSpeed_Modifier
  (params (Key :type Key%20Structure :default "None"))
  ;[1 1 1] Move
  ;;[1 1 1] Speed Modifier
  (:Pressed
    (Variables|Move|SetSpeedModifier 2.0))
  (:Released
    (Variables|Move|SetSpeedModifier 1.0)))

(event Input|ActionEvents|InputActionPan
  (params (Key :type Key%20Structure :default "None"))
  (bind _bp_camera (Variables|Default|GetBP_Camera))
  (bind _returnvalue (Transformation|GetActorRotation _bp_camera))
  (bind (_roll _pitch _yaw) (Math|Rotator|BreakRotator _returnvalue))
  ;[1 1 1] camera rotate (x)
  (:Pressed
    (Utilities|FlowControl|Gate true) ; enters at Open
  )
  (:Released
    (Utilities|FlowControl|Gate true) ; enters at Close
  ))

(event Input|ActionEvents|InputActionPan
  (params (Key :type Key%20Structure :default "None"))
  (bind _bp_camera (Variables|Default|GetBP_Camera))
  (bind _returnvalue (Transformation|GetActorRotation _bp_camera))
  (bind (_roll _pitch _yaw) (Math|Rotator|BreakRotator _returnvalue))
  ;[1 1 1] camera rotate (x)
  (:Pressed
    (Utilities|FlowControl|Gate true) ; enters at Open
  )
  (:Released
    (Utilities|FlowControl|Gate true) ; enters at Close
  ))

(event Input|AxisEvents|InputAxisMove_For/Backword
  (params (AxisValue :type Float%20%28single-precision%29))
  (bind _bp_camera (Variables|Default|GetBP_Camera))
  (bind _speedmodifier (Variables|Move|GetSpeedModifier))
  (bind _movespeed (Variables|Move|GetMoveSpeed))
  (bind _returnvalue (Transformation|GetActorTransform _bp_camera))
  (bind _returnvalue_2 (* AxisValue _speedmodifier _movespeed))
  (bind (_location _rotation _scale) (Math|Transform|BreakTransform _returnvalue))
  (bind _returnvalue_3 (Math|Transform|TransformDirection _returnvalue (Math|Vector|MakeVector _returnvalue_2 0.0 0.0)))
  (bind _returnvalue_4 (+ _returnvalue_3 _location))
  (bind _returnvalue_5 (Math|Transform|MakeTransform _returnvalue_4 _rotation _scale))
  (bind (_x _y) (Math|Vector|BreakVector (.location _returnvalue_5)))
  ;[1 1 1] Move
  ;;[1 1 1] 앞 뒤
  (Transformation|SetActorLocation (Variables|Default|GetBP_Camera) (Math|Vector|MakeVector _x _y 1e+01) false false))

(event Input|AxisEvents|InputAxisMove_Left/Right
  (params (AxisValue :type Float%20%28single-precision%29))
  ;[1 1 1] Move
  ;;[1 1 1] 좌우
  (Class|PawnMovementComponent|AddInputVector (Variables|Default|GetFloating%20Pawn%20Movement) (Math|Vector|MakeVector 0.0 AxisValue 0.0) false))

(event Input|MouseEvents|MouseX
  (params (AxisValue :type Float%20%28single-precision%29))
  (bind _bp_camera (Variables|Default|GetBP_Camera))
  (bind _returnvalue (Transformation|GetActorRotation _bp_camera))
  (bind (_roll _pitch _yaw) (Math|Rotator|BreakRotator _returnvalue))
  ;[1 1 1] camera rotate (x)
  (Utilities|FlowControl|Gate true
    (:Exit
      (Transformation|SetActorRotation (Variables|Default|GetBP_Camera) (Math|Rotator|MakeRotator _roll _pitch (+ _yaw AxisValue))))))

(event Input|MouseEvents|MouseY
  (params (AxisValue :type Float%20%28single-precision%29))
  (bind _bp_camera (Variables|Default|GetBP_Camera))
  (bind _returnvalue (Transformation|GetActorRotation _bp_camera))
  (bind (_roll _pitch _yaw) (Math|Rotator|BreakRotator _returnvalue))
  ;[1 1 1] camera rotate (x)
  (Utilities|FlowControl|Gate true
    (:Exit
      (Transformation|SetActorRotation (Variables|Default|GetBP_Camera) (Math|Rotator|MakeRotator _roll (+ _pitch AxisValue) _yaw)))))

(fn ConstructionScript)