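; BP_GSB keeps the in-game clock, tracking the time of day and a day count.
; On BeginPlay it caches the player's BP_Controller, then seeds GameTime in hours from hour, minute and second variables.
; Each Tick passes delta time, game speed and initial time to SetGameTime and stores the returned GameTime and DayCount.
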(event EventBeginPlay
  (Utilities|FlowControl|Sequence
    (:then_0
      (Utilities|ReferenceCast))
    (:then_1
      (Variables|Default|SetGame%20Time (+ (Variables|Clock|Get시간) (/ (Variables|Clock|Get분) 60) (/ (Variables|Clock|Get초) 3600))))))

(event EventTick
  (params (DeltaSeconds :type Float%20%28single-precision%29))
  (bind (_gametime _daycount) (CallFunction|SetGameTime DeltaSeconds (Variables|Default|GetGame%20Speed) (Variables|Default|GetInitial%20Game%20Time%28게임%20시간%29)))
  (Variables|Default|SetGame%20Time _gametime)
  (Variables|Default|SetDay%20Count _daycount))

(fn ConstructionScript)